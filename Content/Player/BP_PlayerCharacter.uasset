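; First-person shooter player character that handles movement input (walk, run, crouch, jump), firing, reloading, fire-mode switching and returning to the main menu.
; On BeginPlay it spawns a BP_Weapon_Master onto the mesh's GripPoint socket and adds the Shooter_HUD.
; Each tick it points the weapon's muzzle rotation at an aim object and interpolates a separate ADS camera toward the weapon's sight camera or back, switching active cameras for aiming.
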(event `InputAction|Weapon Secondary`
  (params (Key :type "Key Structure"))
  ;[1 1 1] Weapon Secondary
  (:`Pressed`
    (`/Engine/EditorBlueprintResources/StandardMacros.IsValid` (`self.Weapon Active`)
      (:`Is Valid`
        (set `self.IsAiming?` true)
        (`self.Aim Down Sights`))))
  (:`Released`
    (`/Engine/EditorBlueprintResources/StandardMacros.IsValid` (`self.Weapon Active`)
      (:`Is Valid`
        (set `self.IsAiming?` false)
        (`self.UnAim`)))))

(event `InputAction|Weapon Reload`
  (params (Key :type "Key Structure"))
  (bind _weapon_active (`self.Weapon Active`))
  (:`Pressed`
    (if (and (`/Game/Blueprints/Weapons/BP_Weapon_Master.CanReload` (`self.Weapon Active`)) (not (`self.IsFiring?`)) (not (`self.IsReloading?`)) (`self.IsItemEquiped?`))
      (set `self.IsReloading?` true)
      (`/Game/Blueprints/Weapons/BP_Weapon_Master.Reload` _weapon_active)
      (`KismetSystemLibrary.Delay` (`/Game/Blueprints/Weapons/BP_Weapon_Master.ReloadDelay` _weapon_active))
      (set `self.IsReloading?` false))))

(event `InputAction|Weapon Mode`
  (params (Key :type "Key Structure"))
  ;[1 1 1] Change Fire Mode/Weapon
  (:`Pressed`
    (`/Game/Blueprints/Weapons/BP_Weapon_Master.Fire Mode Switch` (`self.Weapon Active`))))

(event `self.ReceiveTick`
  (params (DeltaSeconds :type "Float (single-precision)"))
  ;[1 1 1] Tick System
  (`|ExecutionSequence`
    (:`then_0`
      (`self.SetMuzzleRotation`))
    (:`then_1`
      (if (`self.IsAiming?`)
        (`self.Aim Down Sights`)
        (else
          (`self.UnAim`))))))

(event `InputAxis|Rotate_Left_Right`
  (params (AxisValue :type "Float (single-precision)"))
  ;[1 1 1] Mouse Controls
  (`self.AddControllerYawInput` AxisValue))

(event `InputAxis|Forward_Backward`
  (params (AxisValue :type "Float (single-precision)"))
  ;[1 1 1] Keyboard Movement
  (`self.AddMovementInput` (`self.GetActorForwardVector`) AxisValue))

(event `InputAxis|Look_Up_Down`
  (params (AxisValue :type "Float (single-precision)"))
  ;[1 1 1] Mouse Controls
  (`self.AddControllerPitchInput` AxisValue))

(event `InputAxis|Strafe_Left_Right`
  (params (AxisValue :type "Float (single-precision)"))
  ;[1 1 1] Keyboard Movement
  (`self.AddMovementInput` (`self.GetActorRightVector`) AxisValue))

(event `InputAction|Jump`
  (params (Key :type "Key Structure"))
  ;[1 1 1] Keyboard Movement
  (:`Pressed`
    (set `self.JumpMaxHoldTime` (`self.JumpHeight`))
    (`self.Jump`))
  (:`Released`
    (`self.StopJumping`)))

(event `self.ReceiveBeginPlay`
  ;[1 1 1] Spawn Weapon
  (bind _returnvalue (`|SpawnActorFromClass` "/Game/Blueprints/Weapons/BP_Weapon_Master.BP_Weapon_Master_C" (`KismetMathLibrary.MakeTransform` (0.0 0.0 0.0)) "AlwaysSpawn" "OverrideRootScale" null null))
  (bind _output_get (set `self.Weapon Active` _returnvalue))
  (`self.K2_AttachToComponent` (`self.Weapon Active`) (`self.Mesh`) "GripPoint" "SnapToTarget" "SnapToTarget" "SnapToTarget" true)
  (`self.K2_AttachToComponent` _output_get (`self.Mesh`) "GripPoint" "SnapToTarget" "SnapToTarget" "SnapToTarget" true)
  (bind _returnvalue_2 (`|CreateWidget` "/Game/Blueprints/UI/Shooter_HUD.Shooter_HUD_C" (`GameplayStatics.GetPlayerController` 0)))
  (bind _output_get_2 (set `self.HUD` _returnvalue_2))
  (`UserWidget.AddToViewport` _output_get_2 0))

(event `InputAction|Run`
  (params (Key :type "Key Structure"))
  (bind _charactermovement (`self.CharacterMovement`))
  ;[1 1 1] Keyboard Movement
  (:`Pressed`
    (set `CharacterMovementComponent.MaxWalkSpeed` (`self.RunSpeed`) _charactermovement))
  (:`Released`
    (set `CharacterMovementComponent.MaxWalkSpeed` (`self.WalkSpeed`) _charactermovement)))

(event `InputAction|Crouch`
  (params (Key :type "Key Structure"))
  ;[1 1 1] Keyboard Movement
  (:`Pressed`
    (`self.Crouch`))
  (:`Released`
    (`self.UnCrouch`)))

(event `InputAction|Weapon Primary`
  (params (Key :type "Key Structure"))
  (bind _weapon_active (`self.Weapon Active`))
  ;[1 1 1] Weapon Primary
  (:`Pressed`
    (if (`self.Shootable`)
      (`self.SetMuzzleRotation`)
      (`/Game/Blueprints/Weapons/BP_Weapon_Master.StartFire` _weapon_active)
      (set `self.IsFiring?` true)))
  (:`Released`
    (`/Game/Blueprints/Weapons/BP_Weapon_Master.StopFire` _weapon_active)
    (set `self.IsFiring?` false)))

(event `InputAction|Main Menu`
  (params (Key :type "Key Structure"))
  ;[1 1 1] Keyboard Movement
  (:`Pressed`
    (`GameplayStatics.OpenLevel` "Main_Menu")))

(fn `Aim Down Sights`
  (bind _returnvalue (`GameplayStatics.GetWorldDeltaSeconds`))
  (bind _ads_cam (`self.ADS_Cam`))
  (bind _camera (`/Game/Blueprints/Weapons/BP_Weapon_Master.camera` (`self.Weapon Active`)))
  (`ActorComponent.Deactivate` (`self.FPP_Camera`))
  (`ActorComponent.Activate` _ads_cam false)
  (`SceneComponent.K2_SetWorldLocationAndRotation` _ads_cam (`KismetMathLibrary.VInterpTo` (`SceneComponent.K2_GetComponentLocation` _ads_cam) (`SceneComponent.K2_GetComponentLocation` _camera) _returnvalue 15.0) (`KismetMathLibrary.RInterpTo` (`SceneComponent.K2_GetComponentRotation` _ads_cam) (`SceneComponent.K2_GetComponentRotation` _camera) _returnvalue 15.0) false false))

(fn `Idle`)

(fn `SetMuzzleRotation`
  (bind _weapon_active (`self.Weapon Active`))
  (set `/Game/Blueprints/Weapons/BP_Weapon_Master.MuzzleRotation` (`KismetMathLibrary.FindLookAtRotation` (`SceneComponent.GetSocketLocation` (`/Game/Blueprints/Objects/BP_Object_Master.SkeletalMesh` _weapon_active) "Muzzle") (`SceneComponent.K2_GetComponentLocation` (`self.AimObjectFPP`))) _weapon_active))

(fn `UnAim`
  (bind _returnvalue (`GameplayStatics.GetWorldDeltaSeconds`))
  (bind _ads_cam (`self.ADS_Cam`))
  (bind _fpp_camera (`self.FPP_Camera`))
  (bind _returnvalue_2 (`SceneComponent.K2_GetComponentLocation` _ads_cam))
  (bind (_returnvalue_location _returnvalue_rotation) (`KismetMathLibrary.BreakTransform` (`SceneComponent.K2_GetComponentToWorld` _fpp_camera)))
  (`SceneComponent.K2_SetWorldLocationAndRotation` _ads_cam (`KismetMathLibrary.VInterpTo` _returnvalue_2 _returnvalue_location _returnvalue 15.0) (`KismetMathLibrary.RInterpTo` (`SceneComponent.K2_GetComponentRotation` _ads_cam) _returnvalue_rotation _returnvalue 15.0) false false)
  (if (== _returnvalue_2 _returnvalue_location :`ErrorTolerance` 0.01)
    (`ActorComponent.Deactivate` _ads_cam)
    (`ActorComponent.Activate` _fpp_camera false)))

(fn `UserConstructionScript`)