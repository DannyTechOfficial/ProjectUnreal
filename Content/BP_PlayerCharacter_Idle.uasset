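; BP_PlayerCharacter_Idle is a player character with mouse look, movement, jump, run, crouch, weapon fire and a main-menu key.
; BeginPlay spawns BP_Weapon_Idle, but sets WeaponActive to None rather than the spawned actor before the GripPoint attach.
; Run swaps walk speed, and JumpHeight feeds jump hold time.
; When Shootable, firing turns WeaponActive's muzzle toward AimObjectFPP before calling StartFire.
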(event `InputAxis|Rotate_Left_Right`
  (params (AxisValue :type "Float (single-precision)"))
  ;[1 1 1] Mouse Controls
  (`self.AddControllerYawInput` AxisValue))

(event `InputAxis|Forward_Backward`
  (params (AxisValue :type "Float (single-precision)"))
  ;[1 1 1] Keyboard Movement
  (`self.AddMovementInput` (`self.GetActorForwardVector`) AxisValue))

(event `InputAxis|Look_Up_Down`
  (params (AxisValue :type "Float (single-precision)"))
  ;[1 1 1] Mouse Controls
  (`self.AddControllerPitchInput` AxisValue))

(event `InputAxis|Strafe_Left_Right`
  (params (AxisValue :type "Float (single-precision)"))
  ;[1 1 1] Keyboard Movement
  (`self.AddMovementInput` (`self.GetActorRightVector`) AxisValue))

(event `InputAction|Jump`
  (params (Key :type "Key Structure"))
  ;[1 1 1] Keyboard Movement
  (:`Pressed`
    (set `self.JumpMaxHoldTime` (`self.JumpHeight`))
    (`self.Jump`))
  (:`Released`
    (`self.StopJumping`)))

(event `self.ReceiveBeginPlay`
  (`|SpawnActorFromClass` "/Game/BP_Weapon_Idle.BP_Weapon_Idle_C" (`KismetMathLibrary.MakeTransform` (0.0 0.0 0.0)) "AlwaysSpawn" "OverrideRootScale" null null)
  (bind _output_get (set `self.Weapon Active` null))
  (`self.K2_AttachToComponent` (`self.Weapon Active`) (`self.Mesh`) "GripPoint" "SnapToTarget" "SnapToTarget" "SnapToTarget" true)
  (`self.K2_AttachToComponent` _output_get (`self.Mesh`) "GripPoint" "SnapToTarget" "SnapToTarget" "SnapToTarget" true))

(event `InputAction|Run`
  (params (Key :type "Key Structure"))
  (bind _charactermovement (`self.CharacterMovement`))
  ;[1 1 1] Keyboard Movement
  (:`Pressed`
    (set `CharacterMovementComponent.MaxWalkSpeed` (`self.RunSpeed`) _charactermovement))
  (:`Released`
    (set `CharacterMovementComponent.MaxWalkSpeed` (`self.WalkSpeed`) _charactermovement)))

(event `InputAction|Weapon Primary`
  (params (Key :type "Key Structure"))
  (:`Pressed`
    (if (`self.Shootable`)
      (`self.SetMuzzleRotation`)
      (`/Game/Blueprints/Weapons/BP_Weapon_Master.StartFire` (`self.Weapon Active`)))))

(event `InputAction|Crouch`
  (params (Key :type "Key Structure"))
  ;[1 1 1] Keyboard Movement
  (:`Pressed`
    (`self.Crouch`))
  (:`Released`
    (`self.UnCrouch`)))

(event `InputAction|Main Menu`
  (params (Key :type "Key Structure"))
  ;[1 1 1] Keyboard Movement
  (:`Pressed`
    (`GameplayStatics.OpenLevel` "Main_Menu")))

(fn `Idle`)

(fn `SetMuzzleRotation`
  (bind _weapon_active (`self.Weapon Active`))
  (set `/Game/Blueprints/Weapons/BP_Weapon_Master.MuzzleRotation` (`KismetMathLibrary.FindLookAtRotation` (`SceneComponent.GetSocketLocation` (`/Game/Blueprints/Objects/BP_Object_Master.SkeletalMesh` _weapon_active) "Muzzle") (`SceneComponent.K2_GetComponentLocation` (`self.AimObjectFPP`))) _weapon_active))

(fn `UserConstructionScript`)